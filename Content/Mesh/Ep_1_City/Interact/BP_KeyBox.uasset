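; BP_KeyBox is a one-time interactable crate that adds to the first-person character's BoxCount.
; Interact swaps the crate to its open mesh, increments the count with debug prints, and also moves the world origin to the crate's location.
; The EToInteract prompt turns toward the camera every tick.
; Player overlap with BoxCollision shows the prompt, and end overlap also sets it visible, so it is never hidden here.
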(event `self.ReceiveBeginPlay`
  (bind _asbp_first_person_character (cast `/Game/FirstPerson/Blueprints/BP_FirstPersonCharacter` (`GameplayStatics.GetPlayerCharacter` 0)))
  (set `self.As BP First Person Character` _asbp_first_person_character))

(event `/Game/Mesh/Ep_1_City/Interact/InteractInterface.Interact`
  (bind _box (`self.Box`))
  (`/Engine/EditorBlueprintResources/StandardMacros.DoOnce` false
    (:`Completed`
      (`KismetSystemLibrary.PrintString` "Hello")
      (`StaticMeshComponent.SetStaticMesh` _box "/Game/Mesh/Ep_1_City/ResistanceSquad/crates_set_ind_crate_03_open.crates_set_ind_crate_03_open")
      (`GameplayStatics.SetWorldOriginLocation` (`KismetMathLibrary.FTruncVector` (`SceneComponent.K2_GetComponentLocation` _box)))
      (bind _result (`/Engine/EditorBlueprintResources/StandardMacros.IncrementInt` (`/Game/FirstPerson/Blueprints/BP_FirstPersonCharacter.BoxCount` (`self.As BP First Person Character`)))
        (:`  `
          (`KismetSystemLibrary.PrintString` (`KismetStringLibrary.Conv_IntToString` _result)))))))

(event `self.ReceiveTick`
  (params (DeltaSeconds :type "Float (single-precision)"))
  (bind _e_tointeract (`self.E_toInteract`))
  (`SceneComponent.K2_SetWorldRotation` _e_tointeract (`KismetMathLibrary.FindLookAtRotation` (`SceneComponent.K2_GetComponentLocation` _e_tointeract) (`SceneComponent.K2_GetComponentLocation` (`PlayerCameraManager.TransformComponent` (`GameplayStatics.GetPlayerCameraManager` 0)))) false false))

(event `self.BoxCollision.OnComponentBeginOverlap`
  (params (OverlappedComponent :type "PrimitiveComponent Object Reference") (OtherActor :type "Actor Object Reference") (OtherComp :type "PrimitiveComponent Object Reference") (OtherBodyIndex :type Integer) (bFromSweep :type Boolean) (SweepResult :type "HitResult Structure (by ref)"))
  (if (== OtherActor (`GameplayStatics.GetPlayerCharacter` 0))
    (`SceneComponent.SetVisibility` (`self.E_toInteract`) true false)))

(event `self.BoxCollision.OnComponentEndOverlap`
  (params (OverlappedComponent :type "PrimitiveComponent Object Reference") (OtherActor :type "Actor Object Reference") (OtherComp :type "PrimitiveComponent Object Reference") (OtherBodyIndex :type Integer))
  (if (== (`GameplayStatics.GetPlayerCharacter` 0) OtherActor)
    (`SceneComponent.SetVisibility` (`self.E_toInteract`) true false)))

(fn `UserConstructionScript`)