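; BP_AntiAi is an AI pawn that roams at random and moves toward any pawn it sees.
; Roaming starts on BeginPlay, picking reachable points nearby and repeating after each successful move.
; PawnSensing redirects movement to the seen pawn, and a retriggerable delay resumes roaming shortly after sightings stop.
; A sphere overlap with the first-person character only prints "Run!", while the BP_EnemyAi lookup logic is unfinished.
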(event `self.ReceiveBeginPlay`
  (`self.Random Roan`))

(event `Random Roan`
  (`|AIMoveTo` self (`NavigationSystemV1.K2_GetRandomReachablePointInRadius` (`self.K2_GetActorLocation`) 2500.0 null null) null
    (:`OnSuccess`
      (`self.Random Roan`))))

(event `self.PawnSensing.OnSeePawn`
  (params (Pawn :type "Pawn Object Reference"))
  (`|ExecutionSequence`
    (:`then_0`
      (`|AIMoveTo` self (0.0 0.0 0.0) Pawn))
    (:`then_1`
      (`KismetSystemLibrary.RetriggerableDelay` 1.0)
      (`self.Random Roan`))))

(event `self.Sphere.OnComponentBeginOverlap`
  (params (OverlappedComponent :type "PrimitiveComponent Object Reference") (OtherActor :type "Actor Object Reference") (OtherComp :type "PrimitiveComponent Object Reference") (OtherBodyIndex :type Integer) (bFromSweep :type Boolean) (SweepResult :type "HitResult Structure (by ref)"))
  (cast `/Game/FirstPerson/Blueprints/BP_FirstPersonCharacter` OtherActor)
  (`KismetSystemLibrary.PrintString` "Run!"))

(event `IDK`
  (`|ExecutionSequence`
    (:`then_0`
      (`/Engine/EditorBlueprintResources/StandardMacros.IsValid` (`self.Input Object`)))
    (:`then_1`
      (bind _outactors (`GameplayStatics.GetAllActorsOfClass` "/Game/AI/BP_EnemyAi.BP_EnemyAi_C")))))

(fn `UserConstructionScript`)