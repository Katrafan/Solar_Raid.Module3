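; Ranged rifle enemy that plays a shoot montage, fires at its target through BPCAttacks on an anim notify, then signals attack end.
; Player gun projectile overlaps apply damage, which lowers health shown on a widget bar turned toward the camera every tick.
; At zero health it ragdolls with an upward impulse and particle effect, spawns a BP_SunSphere, then destroys itself.
; Helper functions supply movement speeds and ideal combat range.
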(event `self.ReceiveBeginPlay`
  (`parent.ReceiveBeginPlay`))

(event `self.Attack`
  (params (AttackTarget :type "Actor Object Reference"))
  ;[1 1 1] Fire Rifle
  (`parent.Attack` AttackTarget)
  (bind _notifyname (`|PlayMontage` (`self.Mesh`) "/Game/AI_OLD/AI_Animations/Rebelled/Rebel_Anim_Rig_Shoot_Montage.Rebel_Anim_Rig_Shoot_Montage")
    (:`OnCompleted`
      (`self.EnemyAttackEnd` AttackTarget :!label _label))
    (:`OnInterrupted`
      (goto _label))
    (:`OnNotifyBegin`
      (switch `name` _notifyname
        (:`Fire`
          (`/Game/Attacks/BPC_Attacks.FireBullet` (`self.BPC_Attacks`) (`self.K2_GetActorLocation`) (`self.K2_GetActorLocation` AttackTarget) (make `/Game/DamageSystem/S_DamageInfo` 10.0 "NewEnumerator2" "NewEnumerator0" false true)))))))

(event `self.ReceiveTick`
  (params (DeltaSeconds :type "Float (single-precision)"))
  (bind _healthbar (`self.HealthBar`))
  ;[0.9647 0.227 1] Отображение здоровья
  (bind _aswb_enemy_health (cast `/Game/Widgets/AI/WB_EnemyHealth` (`WidgetComponent.GetWidget` (`self.HealthBar`))))
  (bind _output_get (set `self.WB Enemy Health` _aswb_enemy_health))
  (set `/Game/Widgets/AI/WB_EnemyHealth.CurrentEnHealth` (`self.CurrentEnHealth`) _output_get)
  (set `/Game/Widgets/AI/WB_EnemyHealth.MaxEnHealth` (`self.MaxEnHealth`) _output_get)
  (`SceneComponent.K2_SetWorldRotation` _healthbar (`KismetMathLibrary.FindLookAtRotation` (`SceneComponent.K2_GetComponentLocation` _healthbar) (`SceneComponent.K2_GetComponentLocation` (`PlayerCameraManager.TransformComponent` (`GameplayStatics.GetPlayerCameraManager` 0)))) false false))

(event `self.CapsuleComponent.OnComponentBeginOverlap`
  (params (OverlappedComponent :type "PrimitiveComponent Object Reference") (OtherActor :type "Actor Object Reference") (OtherComp :type "PrimitiveComponent Object Reference") (OtherBodyIndex :type Integer) (bFromSweep :type Boolean) (SweepResult :type "HitResult Structure (by ref)"))
  ;[0.9647 0.227 1] Получение урона
  (cast `/Game/FirstPerson/Blueprints/BP_ShootGunProjectile` OtherActor)
  (`GameplayStatics.ApplyDamage` self 0.5))

(event `self.ReceiveAnyDamage`
  (params (Damage :type "Float (single-precision)") (DamageType :type "DamageType Object Reference") (InstigatedBy :type "Controller Object Reference") (DamageCauser :type "Actor Object Reference"))
  (bind _mesh (`self.Mesh`))
  ;[0.9647 0.227 1] Размер урона и смерть
  (bind _output_get (set `self.CurrentEnHealth` (- (`self.CurrentEnHealth`) (* Damage 50.0))))
  (`/Game/Widgets/AI/WB_EnemyHealth.Update En Health` (`self.WB Enemy Health`) (`KismetMathLibrary.Clamp` _output_get 0 (`self.MaxEnHealth`)))
  (if (<= (`self.CurrentEnHealth`) 0)
    (`GameplayStatics.SpawnEmitterAttached` null (`self.CapsuleComponent`))
    (`PrimitiveComponent.SetSimulatePhysics` _mesh true)
    (`PrimitiveComponent.AddImpulse` _mesh (0.0 0.0 1000.0) "None" false)
    (`|SpawnActorFromClass` "/Game/FirstPerson/Blueprints/Guns/SunSphere/BP_SunSphere.BP_SunSphere_C" (`self.GetTransform`) "Undefined" "MultiplyWithRoot" null null)
    (`KismetSystemLibrary.Delay` 2.0)
    (`self.K2_DestroyActor`)))

(fn `GetIdealRange`
  (returns (AttackRadius :type "Float (double-precision)") (DefendRadius :type "Float (double-precision)"))
  (return 600.0 600.0))

(fn `SetMovementSpeed`
  (params (Speed :type "/Game/RabbitEnemies/AI/Enums/E_MovementSpeed Enum" :default "NewEnumerator0"))
  (returns (SpeedValue :type "Float (double-precision)"))
  (bind _output_get (set `CharacterMovementComponent.MaxWalkSpeed` (select `/Game/RabbitEnemies/AI/Enums/E_MovementSpeed` Speed :`NewEnumerator1` 200.0 :`NewEnumerator2` 300.0 :`NewEnumerator3` 500.0 :!type "Float (single-precision)") (`self.CharacterMovement`)))
  (return _output_get))

(fn `UserConstructionScript`
  (`parent.UserConstructionScript`))