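; Melee enemy AI Blueprint that handles a sphere-trace attack, built on a parent class.
; EnAttack plays the citizen attack montage, and a montage notify triggers a forward sphere trace for Pawns with debug drawing.
; The hit actor receives damage through a TakeDamage message carrying a damage struct.
; Montage completion or interruption calls AttackEnd with the target; the parent BeginPlay call is disabled.
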(event `/Game/AI_OLD/Ai_Control/BPI_EnemyAiOLD.EnAttack`
  (params (AttackTarget :type "Actor Object Reference"))
  (bind _returnvalue (`self.K2_GetActorLocation`))
  (bind _notifyname (`|PlayMontage` (`self.Mesh`) "/Game/AI_OLD/AI_Animations/Citizen_/Citizen_Anim_Attack_Montage.Citizen_Anim_Attack_Montage") ; Сюда анимацию атаки
    (:`OnCompleted`
      (`/Game/AI_OLD/Ai_Control/BPI_EnemyAiOLD.AttackEnd` AttackTarget :!label _label))
    (:`OnInterrupted`
      (goto _label))
    (:`OnNotifyBegin`
      (switch `name` _notifyname
        (:`Slash Trace`
          (bind (_outhit _returnvalue_2) (`KismetSystemLibrary.SphereTraceSingleForObjects` :`Start` _returnvalue :`End` (+ _returnvalue (* (`self.GetActorForwardVector`) 200.0)) :`Radius` 100.0 :`ObjectTypes` (`|MakeArray` "ObjectTypeQuery3" :!type "EObjectTypeQuery Enum") :`DrawDebugType` "ForDuration"))
          (if _returnvalue_2
            (message `/Game/DamageSystem/BPI_Damagable.TakeDamage` (`.HitActor` (`GameplayStatics.BreakHitResult` _outhit)) (make `/Game/DamageSystem/S_DamageInfo` 20.0 "NewEnumerator1") self)))))))

(fn `UserConstructionScript`
  (`parent.UserConstructionScript`))