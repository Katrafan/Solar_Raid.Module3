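; Ranged enemy AI character that plays a ghost sound on spawn, sets walk speed by movement state and supplies attack and defend ranges.
; Attacking starts a shoot montage and spawns BP_VacuumBoom at the gun socket, oriented by the player camera rather than the enemy's aim.
; A montage notify also damages the controller's AttackTarget after a zero-length trace at its location finds no hit.
; Montage completion or interruption calls AttackEnd.
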(event `self.ReceiveBeginPlay`
  (`parent.ReceiveBeginPlay`)
  (for _ (range 1)
    (`GameplayStatics.PlaySoundAtLocation` "/Game/Music/Glitch/ghosts.ghosts" (`self.K2_GetActorLocation`) (struct) 1.0 1.0 0.0 null null null null)))

(event `/Game/AI_OLD/Ai_Control/BPI_EnemyAiOLD.EnAttack`
  (params (AttackTarget :type "Actor Object Reference"))
  (bind _notifyname (`|PlayMontage` (`self.Mesh`) "/Game/AI_OLD/AI_Animations/Rebelled/Rebel_Anim_Rig_Shoot_Montage.Rebel_Anim_Rig_Shoot_Montage")
    (:`then`
      (`self.RangedAttck`))
    (:`OnCompleted`
      (`/Game/AI_OLD/Ai_Control/BPI_EnemyAiOLD.AttackEnd` AttackTarget :!label _label))
    (:`OnInterrupted`
      (goto _label))
    (:`OnNotifyBegin`
      (switch `name` _notifyname
        (:`Fire`
          (bind _asaic_enemy_ai (cast `/Game/AI_OLD/Ai_Control/AIC_EnemyAi` (`AIBlueprintHelperLibrary.GetAIController` self)))
          (bind _attack_target (`/Game/AI_OLD/Ai_Control/AIC_EnemyAi.Attack Target` _asaic_enemy_ai)
            (:`then`
              (bind _returnvalue (`self.K2_GetActorLocation` _attack_target))
              (bind (_outhits _returnvalue_2) (`KismetSystemLibrary.LineTraceMulti` :`Start` _returnvalue :`End` _returnvalue :`TraceChannel` "TraceTypeQuery1" :`DrawDebugType` "ForDuration"))
              (if (not _returnvalue_2)
                (message `/Game/DamageSystem/BPI_Damagable.TakeDamage` _attack_target (make `/Game/DamageSystem/S_DamageInfo` 20.0 "NewEnumerator2") null)))
            (:`else`)))))))

(event `RangedAttck`
  (bind _returnvalue (`PlayerCameraManager.GetCameraRotation` (`GameplayStatics.GetPlayerCameraManager` 0)))
  (`|SpawnActorFromClass` "/Game/FirstPerson/Blueprints/BP_VacuumBoom.BP_VacuumBoom_C" (`KismetMathLibrary.MakeTransform` (+ (`SceneComponent.GetSocketLocation` (`self.Mesh`) "gun") (`KismetMathLibrary.GreaterGreater_VectorRotator` (`self.ProjectileOffset`) _returnvalue)) _returnvalue) "Undefined" "OverrideRootScale" null null))

(fn `Get Ideal Range`
  (returns (AttackRadius :type "Float (double-precision)") (DefendRadius :type "Float (double-precision)"))
  (return 2000.0 600.0))

(fn `SetMovementSpeed`
  (params (Speed :type "/Game/AI_OLD/Ai_Control/Enams/E_MovementSpeed Enum" :default "NewEnumerator0"))
  (returns (SpeedValue :type "Float (double-precision)"))
  (bind _output_get (set `CharacterMovementComponent.MaxWalkSpeed` (select `/Game/AI_OLD/Ai_Control/Enams/E_MovementSpeed` Speed :`NewEnumerator1` 200.0 :`NewEnumerator2` 400.0 :`NewEnumerator3` 700.0 :!type "Float (single-precision)") (`self.CharacterMovement`)))
  (return _output_get))

(fn `UserConstructionScript`
  (`parent.UserConstructionScript`))