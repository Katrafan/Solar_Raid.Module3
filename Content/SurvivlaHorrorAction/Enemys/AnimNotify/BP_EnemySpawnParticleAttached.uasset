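; Anim notify that spawns power-attack effects on a BP_Enemy during an animation.
; It attaches both a Cascade emitter and a Niagara system to a configurable bone on the enemy's mesh, with offset and rotation; scale applies only to the emitter.
; It stores both components on the enemy as its power-attack effect references and plays a sound at the enemy's location.
; Owners that are not BP_Enemy are ignored.
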(fn `Received_Notify`
  (params (MeshComp :type "SkeletalMeshComponent Object Reference") (Animation :type "AnimSequenceBase Object Reference") (EventReference :type "AnimNotifyEventReference Structure (by ref)"))
  (returns (ReturnValue :type Boolean))
  (bind _asbp_enemy (cast `/Game/SurvivlaHorrorAction/Enemys/BP_Enemy` (`ActorComponent.GetOwner` MeshComp)))
  (bind _mesh (`Character.Mesh` _asbp_enemy))
  (bind _returnvalue (`GameplayStatics.SpawnEmitterAttached` (`self.Emitter Template`) _mesh (`self.BoneName`) (`self.AdditionalLocation`) (`self.Rotation`) (`self.Scale`) (`self.Location Type`)))
  (set `/Game/SurvivlaHorrorAction/Enemys/BP_Enemy.ParticleEffectForPowerAttack` _returnvalue _asbp_enemy)
  (bind _returnvalue_2 (`NiagaraFunctionLibrary.SpawnSystemAttached` (`self.System Template`) _mesh (`self.BoneName`) (`self.AdditionalLocation`) (`self.Rotation`) (`self.Location Type`)))
  (set `/Game/SurvivlaHorrorAction/Enemys/BP_Enemy.NiagaraEffectForPowerAttack` _returnvalue_2 _asbp_enemy)
  (`GameplayStatics.PlaySoundAtLocation` (`self.Sound`) (`Actor.K2_GetActorLocation` _asbp_enemy) (struct) 1.0 1.0 0.0 null null null null)
  (return false))