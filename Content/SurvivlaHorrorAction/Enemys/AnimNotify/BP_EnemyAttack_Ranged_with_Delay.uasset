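; Anim notify that triggers a delayed ranged attack on the BP_Enemy that owns the animated mesh.
; It passes its trace shape, damage, delay, friendly-kill and debug settings to EnemyAttackWithDelay, negating the trace angle when ClockDirection is off.
; Helper functions look up bullet-hit Niagara, particle, decal and sound effects by surface, but the notify itself never calls them.
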(fn `HitDecal`
  (params (Surface :type "EPhysicalSurface Enum" :default "SurfaceType_Default"))
  (returns (Value1 :type "MaterialInstance Object Reference"))
  (return (`BlueprintMapLibrary.Map_Find` (`.BulletHitParticleEffect_11_316A98754E7227CD25349FB9E9BF1C32` (break `/Game/SurvivlaHorrorAction/GameSettings/Struct_BulletHitDecalEffect` (`/Game/SurvivlaHorrorAction/Functions/BFL_Functions.F_Game bullet hit decal effects`))) Surface)))

(fn `HitNiagara`
  (params (Surface :type "EPhysicalSurface Enum" :default "SurfaceType_Default"))
  (returns (Value :type "NiagaraSystem Object Reference"))
  (return (`BlueprintMapLibrary.Map_Find` (`.BulletHitParticleEffect_8_316A98754E7227CD25349FB9E9BF1C32` (break `/Game/SurvivlaHorrorAction/GameSettings/Struct_BulletHitNiagaraEffect` (`/Game/SurvivlaHorrorAction/Functions/BFL_Functions.F_Game bullet hit niagara effects`))) Surface)))

(fn `HitParticle`
  (params (Surface :type "EPhysicalSurface Enum" :default "SurfaceType_Default"))
  (returns (Value :type "ParticleSystem Object Reference"))
  (return (`BlueprintMapLibrary.Map_Find` (`.BulletHitParticleEffect_7_316A98754E7227CD25349FB9E9BF1C32` (break `/Game/SurvivlaHorrorAction/GameSettings/Struct_BulletHitParticleEffect` (`/Game/SurvivlaHorrorAction/Functions/BFL_Functions.F_Game bullet hit paricle effects`))) Surface)))

(fn `Hitsound`
  (params (Surface :type "EPhysicalSurface Enum" :default "SurfaceType_Default"))
  (returns (Value :type "SoundBase Object Reference"))
  (return (`BlueprintMapLibrary.Map_Find` (`.BulletHitParticleEffect_9_316A98754E7227CD25349FB9E9BF1C32` (break `/Game/SurvivlaHorrorAction/GameSettings/Struct_BulletHitSoundEffect` (`/Game/SurvivlaHorrorAction/Functions/BFL_Functions.F_Game bullet hit sound effects`))) Surface)))

(fn `Received_Notify`
  (params (MeshComp :type "SkeletalMeshComponent Object Reference") (Animation :type "AnimSequenceBase Object Reference") (EventReference :type "AnimNotifyEventReference Structure (by ref)"))
  (returns (ReturnValue :type Boolean))
  (bind _asbp_enemy (cast `/Game/SurvivlaHorrorAction/Enemys/BP_Enemy` (`ActorComponent.GetOwner` MeshComp)))
  (`/Game/SurvivlaHorrorAction/Enemys/BP_Enemy.EnemyAttackWithDelay` _asbp_enemy (`self.Forward`) (`self.Right`) (`self.Up`) (`self.TraceCounts`) (`self.TraceSize`) (`KismetMathLibrary.SelectFloat` (`self.TraceAngle`) (* (`self.TraceAngle`) -1.0) (`self.ClockDirection?`)) (`self.TraceDistance`) (`self.Additional Angle`) (`self.Draw Debug Type`) (`self.Base Damage`) (`self.CanKillEnemyToo?`) (`self.Delay`))
  (return false))