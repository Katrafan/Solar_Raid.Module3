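; Anim notify that lets an enemy inflict abnormal conditions on survival horror characters during an animation.
; On the server, it fires a fan of sphere traces from a configurable offset, centred on the enemy's forward direction plus an extra angle.
; Hit characters receive a request with condition, recovery time and success ratio.
; The enemy's AbnormalActor caches the last hit to skip consecutive repeats, resetting after the loop.
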(fn `Received_Notify`
  (params (MeshComp :type "SkeletalMeshComponent Object Reference") (Animation :type "AnimSequenceBase Object Reference") (EventReference :type "AnimNotifyEventReference Structure (by ref)"))
  (returns (ReturnValue :type Boolean))
  (if (`KismetSystemLibrary.IsServer`)
    (bind _asbp_enemy (cast `/Game/SurvivlaHorrorAction/Enemys/BP_Enemy` (`ActorComponent.GetOwner` MeshComp)))
    (for _index (range (`self.TraceCounts`))
      (`SubmixEffectDelayStatics.SetDelayLength` (make `SubmixEffectDelaySettings` 2000.0) 1.0)
      (bind _returnvalue (+ (`Actor.K2_GetActorLocation` _asbp_enemy) (+ (* (`Actor.GetActorForwardVector` _asbp_enemy) (`self.Forward`)) (* (`Actor.GetActorRightVector` _asbp_enemy) (`self.Right`)) (* (`Actor.GetActorUpVector` _asbp_enemy) (`self.Up`)))))
      (bind (_outhit _returnvalue_2) (`KismetSystemLibrary.SphereTraceSingle` _returnvalue (+ _returnvalue (* (`KismetMathLibrary.GreaterGreater_VectorRotator` (`Actor.GetActorForwardVector` _asbp_enemy) (`KismetMathLibrary.MakeRotator` 0.0 0.0 (+ (* (`KismetMathLibrary.Conv_IntToDouble` _index) (`self.TraceAngle`)) (+ (/ (* (`KismetMathLibrary.Conv_IntToDouble` (- (`self.TraceCounts`) 1)) (`self.TraceAngle`)) -2.0) (`self.AdditionalAngle`))))) (`self.TraceDistance`))) (`self.TraceSize`) "TraceTypeQuery1" false (`|MakeArray` _asbp_enemy :!type "Actor Object Reference") (`self.Draw Debug Type`)))
      (if _returnvalue_2
        (bind (_bblockinghit _binitialoverlap _time _distance _location _impactpoint _normal _impactnormal _physmat _hitactor) (`GameplayStatics.BreakHitResult` _outhit))
        (if (not (== (`/Game/SurvivlaHorrorAction/Enemys/BP_Enemy.AbnormalActor` _asbp_enemy) _hitactor))
          (set `/Game/SurvivlaHorrorAction/Enemys/BP_Enemy.AbnormalActor` _hitactor _asbp_enemy)
          (bind _asbp_survival_horror_character (cast `/Game/SurvivlaHorrorAction/Demo/BP_SurvivalHorrorCharacter` _hitactor))
          (`/Game/SurvivlaHorrorAction/Demo/BP_SurvivalHorrorCharacter.RequestSetAbnormalConditions` _asbp_survival_horror_character (`self.Conditions`) (`self.Recovery Time`) (`self.Success Ratio`)))))
    (set `/Game/SurvivlaHorrorAction/Enemys/BP_Enemy.AbnormalActor` null _asbp_enemy)))