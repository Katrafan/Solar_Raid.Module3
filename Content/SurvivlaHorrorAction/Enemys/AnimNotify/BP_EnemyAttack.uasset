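; Anim notify that performs an enemy's attack hit check, skipped when the limbs or head that attack type needs are blown off.
; It fans sphere traces from an offset, filtering out rolling players, dead enemies, destroyed vehicles and knocked-down followers.
; Hits spawn surface-based particles, decals and sound, swapped for guard effects when enemies or players block non-power attacks.
; The server applies scaled damage, passing the montage index to character victims.
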(fn `Hit Niagara`
  (params (Surface :type "EPhysicalSurface Enum" :default "SurfaceType_Default") (HItActor :type "Actor Object Reference"))
  (returns (Value :type "NiagaraSystem Object Reference"))
  (bind _value (`BlueprintMapLibrary.Map_Find` (`.BulletHitParticleEffect_8_316A98754E7227CD25349FB9E9BF1C32` (break `/Game/SurvivlaHorrorAction/GameSettings/Struct_BulletHitNiagaraEffect` (`/Game/SurvivlaHorrorAction/Functions/BFL_Functions.F_Game bullet hit niagara effects`))) Surface))
  (bind _asbp_enemy (cast `/Game/SurvivlaHorrorAction/Enemys/BP_Enemy` HItActor)
    (:`then`
      (return (select `bool` (and (`/Game/SurvivlaHorrorAction/Enemys/BP_Enemy.Guard?` _asbp_enemy) (!= (`self.Damage Type Class`) "/Game/SurvivlaHorrorAction/Blueprints/DamageType/BP_PowerAttack.BP_PowerAttack_C")) :`false` _value :`true` (`/Game/SurvivlaHorrorAction/Enemys/BP_Enemy.GuardNiagara` _asbp_enemy))))
    (:`CastFailed`
      (bind _asbp_survival_horror_character (cast `/Game/SurvivlaHorrorAction/Demo/BP_SurvivalHorrorCharacter` HItActor)
        (:`then`
          (bind ((`WeaponType_75_08CD22A54C4C1C8BDA8A8CBF3808702E` _weapontype) (`BurntScale_301_4343C50D4D84FAC23291D994DC56121E` _burntscale) (`BurntImpulse_304_A69417704F2104E1F13157AE830717B8` _burntimpulse) (`WeaponRightHandTransform_296_F002A4934DA72FBBC97C069E8D18A771` _weaponrighthandtransform) (`GuardNiagaraSystem_239_0224D3C248E37375024849920D151B53` _guardniagarasystem)) (break `/Game/SurvivlaHorrorAction/GameSettings/Struct_Weapons` (`/Game/SurvivlaHorrorAction/Demo/BP_SurvivalHorrorCharacter.CurrentWeaponData` _asbp_survival_horror_character)))
          (return (select `bool` (and (`/Game/SurvivlaHorrorAction/Demo/BP_SurvivalHorrorCharacter.Guard` _asbp_survival_horror_character) (!= (`self.Damage Type Class`) "/Game/SurvivlaHorrorAction/Blueprints/DamageType/BP_PowerAttack.BP_PowerAttack_C")) :`false` _value :`true` (select `bool` (and (`|EnumEquality` _weapontype "NewEnumerator13") (not (`KismetTextLibrary.TextIsEmpty` (`.ItemName_2_5AE7D555463CAE7A9A71FE8D920EC148` (break `/Game/SurvivlaHorrorAction/GameSettings/Struct_Inventory` (`|GetArrayItem` (`/Game/SurvivlaHorrorAction/Demo/BP_SurvivalHorrorCharacter.Inventory` _asbp_survival_horror_character) 42))))) (== (`SceneComponent.GetAttachSocketName` (`/Game/SurvivlaHorrorAction/Demo/BP_SurvivalHorrorCharacter.Shield` _asbp_survival_horror_character)) (`/Game/SurvivlaHorrorAction/Demo/BP_SurvivalHorrorCharacter.ShieldAttachedBone` _asbp_survival_horror_character))) :`false` _guardniagarasystem :`true` (`.GuardNiagaraSystem_239_0224D3C248E37375024849920D151B53` (break `/Game/SurvivlaHorrorAction/GameSettings/Struct_Weapons` (`/Game/SurvivlaHorrorAction/Demo/BP_SurvivalHorrorCharacter.GetNextWeaponData` _asbp_survival_horror_character 42)))))))
        (:`CastFailed`
          (return _value))))))

(fn `Hit Particle`
  (params (Surface :type "EPhysicalSurface Enum" :default "SurfaceType_Default") (HitActor :type "Actor Object Reference"))
  (returns (Value :type "ParticleSystem Object Reference"))
  (bind _value (`BlueprintMapLibrary.Map_Find` (`.BulletHitParticleEffect_7_316A98754E7227CD25349FB9E9BF1C32` (break `/Game/SurvivlaHorrorAction/GameSettings/Struct_BulletHitParticleEffect` (`/Game/SurvivlaHorrorAction/Functions/BFL_Functions.F_Game bullet hit paricle effects`))) Surface))
  (bind _asbp_enemy (cast `/Game/SurvivlaHorrorAction/Enemys/BP_Enemy` HitActor)
    (:`then`
      (return (select `bool` (and (`/Game/SurvivlaHorrorAction/Enemys/BP_Enemy.Guard?` _asbp_enemy) (!= (`self.Damage Type Class`) "/Game/SurvivlaHorrorAction/Blueprints/DamageType/BP_PowerAttack.BP_PowerAttack_C")) :`false` _value :`true` (`/Game/SurvivlaHorrorAction/Enemys/BP_Enemy.GuardParticle` _asbp_enemy))))
    (:`CastFailed`
      (bind _asbp_survival_horror_character (cast `/Game/SurvivlaHorrorAction/Demo/BP_SurvivalHorrorCharacter` HitActor)
        (:`then`
          (bind ((`WeaponType_75_08CD22A54C4C1C8BDA8A8CBF3808702E` _weapontype) (`BurntScale_301_4343C50D4D84FAC23291D994DC56121E` _burntscale) (`BurntImpulse_304_A69417704F2104E1F13157AE830717B8` _burntimpulse) (`WeaponRightHandTransform_296_F002A4934DA72FBBC97C069E8D18A771` _weaponrighthandtransform) (`GuardParticleSystem_236_562139CF4723869540F265A2C1B177A0` _guardparticlesystem)) (break `/Game/SurvivlaHorrorAction/GameSettings/Struct_Weapons` (`/Game/SurvivlaHorrorAction/Demo/BP_SurvivalHorrorCharacter.CurrentWeaponData` _asbp_survival_horror_character)))
          (return (select `bool` (and (`/Game/SurvivlaHorrorAction/Demo/BP_SurvivalHorrorCharacter.Guard` _asbp_survival_horror_character) (!= (`self.Damage Type Class`) "/Game/SurvivlaHorrorAction/Blueprints/DamageType/BP_PowerAttack.BP_PowerAttack_C")) :`false` _value :`true` (select `bool` (and (`|EnumEquality` _weapontype "NewEnumerator13") (not (`KismetTextLibrary.TextIsEmpty` (`.ItemName_2_5AE7D555463CAE7A9A71FE8D920EC148` (break `/Game/SurvivlaHorrorAction/GameSettings/Struct_Inventory` (`|GetArrayItem` (`/Game/SurvivlaHorrorAction/Demo/BP_SurvivalHorrorCharacter.Inventory` _asbp_survival_horror_character) 42))))) (== (`SceneComponent.GetAttachSocketName` (`/Game/SurvivlaHorrorAction/Demo/BP_SurvivalHorrorCharacter.Shield` _asbp_survival_horror_character)) (`/Game/SurvivlaHorrorAction/Demo/BP_SurvivalHorrorCharacter.ShieldAttachedBone` _asbp_survival_horror_character))) :`false` _guardparticlesystem :`true` (`.GuardParticleSystem_236_562139CF4723869540F265A2C1B177A0` (break `/Game/SurvivlaHorrorAction/GameSettings/Struct_Weapons` (`/Game/SurvivlaHorrorAction/Demo/BP_SurvivalHorrorCharacter.GetNextWeaponData` _asbp_survival_horror_character 42)))))))
        (:`CastFailed`
          (return _value))))))

(fn `HitDecal`
  (params (Surface :type "EPhysicalSurface Enum" :default "SurfaceType_Default") (HitActor :type "Actor Object Reference"))
  (returns (Value1 :type "MaterialInstance Object Reference"))
  (bind _value (`BlueprintMapLibrary.Map_Find` (`.BulletHitParticleEffect_11_316A98754E7227CD25349FB9E9BF1C32` (break `/Game/SurvivlaHorrorAction/GameSettings/Struct_BulletHitDecalEffect` (`/Game/SurvivlaHorrorAction/Functions/BFL_Functions.F_Game bullet hit decal effects`))) Surface))
  (bind _asbp_enemy (cast `/Game/SurvivlaHorrorAction/Enemys/BP_Enemy` HitActor)
    (:`then`
      (return (select `bool` (and (`/Game/SurvivlaHorrorAction/Enemys/BP_Enemy.Guard?` _asbp_enemy) (!= (`self.Damage Type Class`) "/Game/SurvivlaHorrorAction/Blueprints/DamageType/BP_PowerAttack.BP_PowerAttack_C")) :`false` _value :`true` (`/Game/SurvivlaHorrorAction/Enemys/BP_Enemy.GuardDecal` _asbp_enemy))))
    (:`CastFailed`
      (bind _asbp_survival_horror_character (cast `/Game/SurvivlaHorrorAction/Demo/BP_SurvivalHorrorCharacter` HitActor)
        (:`then`
          (bind ((`WeaponType_75_08CD22A54C4C1C8BDA8A8CBF3808702E` _weapontype) (`BurntScale_301_4343C50D4D84FAC23291D994DC56121E` _burntscale) (`BurntImpulse_304_A69417704F2104E1F13157AE830717B8` _burntimpulse) (`WeaponRightHandTransform_296_F002A4934DA72FBBC97C069E8D18A771` _weaponrighthandtransform) (`GuardDecal_246_B846D1A84A07727F342FD39893685FB7` _guarddecal)) (break `/Game/SurvivlaHorrorAction/GameSettings/Struct_Weapons` (`/Game/SurvivlaHorrorAction/Demo/BP_SurvivalHorrorCharacter.CurrentWeaponData` _asbp_survival_horror_character)))
          (return (select `bool` (and (`/Game/SurvivlaHorrorAction/Demo/BP_SurvivalHorrorCharacter.Guard` _asbp_survival_horror_character) (!= (`self.Damage Type Class`) "/Game/SurvivlaHorrorAction/Blueprints/DamageType/BP_PowerAttack.BP_PowerAttack_C")) :`false` _value :`true` (select `bool` (and (`|EnumEquality` _weapontype "NewEnumerator13") (not (`KismetTextLibrary.TextIsEmpty` (`.ItemName_2_5AE7D555463CAE7A9A71FE8D920EC148` (break `/Game/SurvivlaHorrorAction/GameSettings/Struct_Inventory` (`|GetArrayItem` (`/Game/SurvivlaHorrorAction/Demo/BP_SurvivalHorrorCharacter.Inventory` _asbp_survival_horror_character) 42))))) (== (`SceneComponent.GetAttachSocketName` (`/Game/SurvivlaHorrorAction/Demo/BP_SurvivalHorrorCharacter.Shield` _asbp_survival_horror_character)) (`/Game/SurvivlaHorrorAction/Demo/BP_SurvivalHorrorCharacter.ShieldAttachedBone` _asbp_survival_horror_character))) :`false` _guarddecal :`true` (`.GuardDecal_246_B846D1A84A07727F342FD39893685FB7` (break `/Game/SurvivlaHorrorAction/GameSettings/Struct_Weapons` (`/Game/SurvivlaHorrorAction/Demo/BP_SurvivalHorrorCharacter.GetNextWeaponData` _asbp_survival_horror_character 42)))))))
        (:`CastFailed`
          (return _value))))))

(fn `Hitsound`
  (params (Surface :type "EPhysicalSurface Enum" :default "SurfaceType_Default") (HitActor :type "Actor Object Reference"))
  (returns (Value :type "SoundBase Object Reference"))
  (bind _value (`BlueprintMapLibrary.Map_Find` (`.BulletHitParticleEffect_9_316A98754E7227CD25349FB9E9BF1C32` (break `/Game/SurvivlaHorrorAction/GameSettings/Struct_BulletHitSoundEffect` (`/Game/SurvivlaHorrorAction/Functions/BFL_Functions.F_Game bullet hit sound effects`))) Surface))
  (bind _asbp_enemy (cast `/Game/SurvivlaHorrorAction/Enemys/BP_Enemy` HitActor)
    (:`then`
      (return (select `bool` (and (`/Game/SurvivlaHorrorAction/Enemys/BP_Enemy.Guard?` _asbp_enemy) (!= (`self.Damage Type Class`) "/Game/SurvivlaHorrorAction/Blueprints/DamageType/BP_PowerAttack.BP_PowerAttack_C")) :`false` _value :`true` (`/Game/SurvivlaHorrorAction/Enemys/BP_Enemy.GuardSound` _asbp_enemy))))
    (:`CastFailed`
      (bind _asbp_survival_horror_character (cast `/Game/SurvivlaHorrorAction/Demo/BP_SurvivalHorrorCharacter` HitActor)
        (:`then`
          (bind ((`WeaponType_75_08CD22A54C4C1C8BDA8A8CBF3808702E` _weapontype) (`BurntScale_301_4343C50D4D84FAC23291D994DC56121E` _burntscale) (`BurntImpulse_304_A69417704F2104E1F13157AE830717B8` _burntimpulse) (`WeaponRightHandTransform_296_F002A4934DA72FBBC97C069E8D18A771` _weaponrighthandtransform) (`GuardSound_245_16678D794E73EF4F893688969E9CE71A` _guardsound)) (break `/Game/SurvivlaHorrorAction/GameSettings/Struct_Weapons` (`/Game/SurvivlaHorrorAction/Demo/BP_SurvivalHorrorCharacter.CurrentWeaponData` _asbp_survival_horror_character)))
          (return (select `bool` (and (`/Game/SurvivlaHorrorAction/Demo/BP_SurvivalHorrorCharacter.Guard` _asbp_survival_horror_character) (!= (`self.Damage Type Class`) "/Game/SurvivlaHorrorAction/Blueprints/DamageType/BP_PowerAttack.BP_PowerAttack_C")) :`false` _value :`true` (select `bool` (and (`|EnumEquality` _weapontype "NewEnumerator13") (not (`KismetTextLibrary.TextIsEmpty` (`.ItemName_2_5AE7D555463CAE7A9A71FE8D920EC148` (break `/Game/SurvivlaHorrorAction/GameSettings/Struct_Inventory` (`|GetArrayItem` (`/Game/SurvivlaHorrorAction/Demo/BP_SurvivalHorrorCharacter.Inventory` _asbp_survival_horror_character) 42))))) (== (`SceneComponent.GetAttachSocketName` (`/Game/SurvivlaHorrorAction/Demo/BP_SurvivalHorrorCharacter.Shield` _asbp_survival_horror_character)) (`/Game/SurvivlaHorrorAction/Demo/BP_SurvivalHorrorCharacter.ShieldAttachedBone` _asbp_survival_horror_character))) :`false` _guardsound :`true` (`.GuardSound_245_16678D794E73EF4F893688969E9CE71A` (break `/Game/SurvivlaHorrorAction/GameSettings/Struct_Weapons` (`/Game/SurvivlaHorrorAction/Demo/BP_SurvivalHorrorCharacter.GetNextWeaponData` _asbp_survival_horror_character 42)))))))
        (:`CastFailed`
          (return _value))))))

(fn `Received_Notify`
  (params (MeshComp :type "SkeletalMeshComponent Object Reference") (Animation :type "AnimSequenceBase Object Reference") (EventReference :type "AnimNotifyEventReference Structure (by ref)"))
  (returns (ReturnValue :type Boolean))
  (bind _asbp_enemy (cast `/Game/SurvivlaHorrorAction/Enemys/BP_Enemy` (`ActorComponent.GetOwner` MeshComp)))
  (switch `/Game/SurvivlaHorrorAction/Enum/Enum_EnemyAttackType` (`self.EnemyAttackType`)
    (:`NewEnumerator23`
      (for _index (range (`self.TraceCounts`)) :!label _label
        (`SubmixEffectDelayStatics.SetDelayLength` (make `SubmixEffectDelaySettings` 2000.0) 1.0)
        (bind _returnvalue (+ (`Actor.K2_GetActorLocation` _asbp_enemy) (+ (* (`Actor.GetActorForwardVector` _asbp_enemy) (`self.Forward`)) (* (`Actor.GetActorRightVector` _asbp_enemy) (`self.Right`)) (* (`Actor.GetActorUpVector` _asbp_enemy) (`self.Up`)))))
        (bind (_outhit _returnvalue_2) (`KismetSystemLibrary.SphereTraceSingle` _returnvalue (+ _returnvalue (* (`KismetMathLibrary.GreaterGreater_VectorRotator` (`Actor.GetActorForwardVector` _asbp_enemy) (`KismetMathLibrary.MakeRotator` 0.0 0.0 (+ (* (`KismetMathLibrary.Conv_IntToDouble` _index) (`self.TraceAngle`)) (+ (/ (* (`KismetMathLibrary.Conv_IntToDouble` (- (`self.TraceCounts`) 1)) (`self.TraceAngle`)) -2.0) (`self.AdditionalAngle`))))) (`self.TraceDistance`))) (`self.TraceSize`) "TraceTypeQuery1" false (`|MakeArray` _asbp_enemy :!type "Actor Object Reference") (`self.Draw Debug Type`)))
        (if _returnvalue_2
          (bind (_bblockinghit _binitialoverlap _time _distance _location _impactpoint _normal _impactnormal _physmat _hitactor _hitcomponent _hitbonename) (`GameplayStatics.BreakHitResult` _outhit))
          (bind _asbp_survival_horror_character (cast `/Game/SurvivlaHorrorAction/Demo/BP_SurvivalHorrorCharacter` _hitactor)
            (:`then`
              (if (== (`/Game/SurvivlaHorrorAction/Enemys/BP_Enemy.AttackTraceHittedActor` _asbp_enemy) _hitactor)
                _
                (elif (not (`/Game/SurvivlaHorrorAction/Demo/BP_SurvivalHorrorCharacter.Rolling?` _asbp_survival_horror_character))
                  (set `/Game/SurvivlaHorrorAction/Enemys/BP_Enemy.AttackTraceHittedActor` _hitactor _asbp_enemy :!label _label_2)
                  (`GameplayStatics.SpawnEmitterAtLocation` (`self.Hit Particle` (`GameplayStatics.GetSurfaceType` _outhit) _hitactor) _location)
                  (`NiagaraFunctionLibrary.SpawnSystemAtLocation` (`self.Hit Niagara` (`GameplayStatics.GetSurfaceType` _outhit) _hitactor) _location)
                  (bind _returnvalue_3 (`GameplayStatics.SpawnDecalAttached` (`self.HitDecal` (`GameplayStatics.GetSurfaceType` _outhit) _hitactor) (10.0 10.0 10.0) _hitcomponent _hitbonename _location (`KismetMathLibrary.Conv_VectorToRotator` _normal) "KeepRelativeOffset" 10.0))
                  (`/Engine/EditorBlueprintResources/StandardMacros.IsValid` _returnvalue_3
                    (:`Is Valid`
                      (`DecalComponent.SetFadeOut` _returnvalue_3 10.0 3.0 false))
                    (:`Is Not Valid`
                      _))
                  (`/Game/SurvivlaHorrorAction/Functions/BFL_Functions.F_PlaySound_At_Location` (`self.Hitsound` (`GameplayStatics.GetSurfaceType` _outhit) _hitactor) _location)
                  (if (`KismetSystemLibrary.IsServer`)
                    (bind _asbp_vehicle (cast `/Game/SurvivlaHorrorAction/Vehicle/BP_Vehicle` _hitactor)
                      (:`then`
                        (message `/Game/SurvivlaHorrorAction/Functions/BPI_Connection.AddDamage` _asbp_enemy (* (`self.Base Damage`) (`/Game/SurvivlaHorrorAction/Enemys/BP_Enemy.AttackDamage` _asbp_enemy)) _asbp_vehicle _asbp_enemy (`self.Damage Type Class`)))
                      (:`CastFailed`
                        (bind _asbp_enemy_2 (cast `/Game/SurvivlaHorrorAction/Enemys/BP_Enemy` _hitactor)
                          (:`then`
                            (bind _randomattackmontageindex (`/Game/SurvivlaHorrorAction/Enemys/BP_Enemy.RandomAttackMontageIndex` _asbp_enemy))
                            (set `/Game/SurvivlaHorrorAction/Enemys/BP_Enemy.HitIndex` _randomattackmontageindex _asbp_enemy_2))
                          (:`CastFailed`
                            (bind _asbp_survival_horror_character_2 (cast `/Game/SurvivlaHorrorAction/Demo/BP_SurvivalHorrorCharacter` _hitactor)
                              (:`then`
                                (set `/Game/SurvivlaHorrorAction/Demo/BP_SurvivalHorrorCharacter.HitIndex` _randomattackmontageindex _asbp_survival_horror_character_2))
                              (:`CastFailed`
                                (bind _asbp_follower (cast `/Game/SurvivlaHorrorAction/Follower/BP_Follower` _hitactor))
                                (set `/Game/SurvivlaHorrorAction/Follower/BP_Follower.HitIndex` _randomattackmontageindex _asbp_follower)))))
                        (`GameplayStatics.ApplyDamage` _hitactor (* (`self.Base Damage`) (`/Game/SurvivlaHorrorAction/Enemys/BP_Enemy.AttackDamage` _asbp_enemy)) null _asbp_enemy (`self.Damage Type Class`))))))))
            (:`CastFailed`
              (bind _asbp_enemy_3 (cast `/Game/SurvivlaHorrorAction/Enemys/BP_Enemy` _hitactor)
                (:`then`
                  (if (not (`/Game/SurvivlaHorrorAction/Enemys/BP_Enemy.Dead?` _asbp_enemy_3))
                    (goto _label_2)))
                (:`CastFailed`
                  (bind _asbp_vehicle_2 (cast `/Game/SurvivlaHorrorAction/Vehicle/BP_Vehicle` _hitactor)
                    (:`then`
                      (if (not (`/Game/SurvivlaHorrorAction/Vehicle/BP_Vehicle.Destroyed` _asbp_vehicle_2))
                        (goto _label_2)))
                    (:`CastFailed`
                      (bind _asbp_follower_2 (cast `/Game/SurvivlaHorrorAction/Follower/BP_Follower` _hitactor))
                      (if (not (`/Game/SurvivlaHorrorAction/Follower/BP_Follower.KnockDown` _asbp_follower_2))
                        (goto _label_2))))))))))
      (set `/Game/SurvivlaHorrorAction/Enemys/BP_Enemy.AttackTraceHittedActor` null _asbp_enemy))
    (:`NewEnumerator24`
      (goto _label))
    (:`NewEnumerator0`
      (if (not (`/Game/SurvivlaHorrorAction/Enemys/BP_Enemy.LUpperArmBlow` _asbp_enemy))
        (goto _label)))
    (:`NewEnumerator4`
      (if (not (`/Game/SurvivlaHorrorAction/Enemys/BP_Enemy.RUpperArmBlow` _asbp_enemy))
        (goto _label)))
    (:`NewEnumerator5`
      (if (not (and (`/Game/SurvivlaHorrorAction/Enemys/BP_Enemy.LUpperArmBlow` _asbp_enemy) (`/Game/SurvivlaHorrorAction/Enemys/BP_Enemy.RUpperArmBlow` _asbp_enemy)))
        (goto _label)))
    (:`NewEnumerator20`
      (if (not (`/Game/SurvivlaHorrorAction/Enemys/BP_Enemy.HeadBlow` _asbp_enemy))
        (goto _label)))))