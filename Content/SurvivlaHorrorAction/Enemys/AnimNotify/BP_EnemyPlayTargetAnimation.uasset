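; Enemy anim notify that makes survival horror characters caught by an attack trace play a counter animation.
; It sweeps a configurable fan of sphere traces from an offset oriented toward the enemy's TargetActor, collecting each character once in the enemy's hit map.
; Each gets a PlayTargetAnimation message with its animation for the enemy's CounterIndex, then the map clears.
; Surface-based bullet-hit effect lookup helpers are defined but unused by the notify.
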(fn `HitDecal`
  (params (Surface :type "EPhysicalSurface Enum" :default "SurfaceType_Default"))
  (returns (Value1 :type "MaterialInstance Object Reference"))
  (return (`BlueprintMapLibrary.Map_Find` (`.BulletHitParticleEffect_11_316A98754E7227CD25349FB9E9BF1C32` (break `/Game/SurvivlaHorrorAction/GameSettings/Struct_BulletHitDecalEffect` (`/Game/SurvivlaHorrorAction/Functions/BFL_Functions.F_Game bullet hit decal effects`))) Surface)))

(fn `HitNiagara`
  (params (Surface :type "EPhysicalSurface Enum" :default "SurfaceType_Default"))
  (returns (Value :type "NiagaraSystem Object Reference"))
  (return (`BlueprintMapLibrary.Map_Find` (`.BulletHitParticleEffect_8_316A98754E7227CD25349FB9E9BF1C32` (break `/Game/SurvivlaHorrorAction/GameSettings/Struct_BulletHitNiagaraEffect` (`/Game/SurvivlaHorrorAction/Functions/BFL_Functions.F_Game bullet hit niagara effects`))) Surface)))

(fn `HitParticle`
  (params (Surface :type "EPhysicalSurface Enum" :default "SurfaceType_Default"))
  (returns (Value :type "ParticleSystem Object Reference"))
  (return (`BlueprintMapLibrary.Map_Find` (`.BulletHitParticleEffect_7_316A98754E7227CD25349FB9E9BF1C32` (break `/Game/SurvivlaHorrorAction/GameSettings/Struct_BulletHitParticleEffect` (`/Game/SurvivlaHorrorAction/Functions/BFL_Functions.F_Game bullet hit paricle effects`))) Surface)))

(fn `Hitsound`
  (params (Surface :type "EPhysicalSurface Enum" :default "SurfaceType_Default"))
  (returns (Value :type "SoundBase Object Reference"))
  (return (`BlueprintMapLibrary.Map_Find` (`.BulletHitParticleEffect_9_316A98754E7227CD25349FB9E9BF1C32` (break `/Game/SurvivlaHorrorAction/GameSettings/Struct_BulletHitSoundEffect` (`/Game/SurvivlaHorrorAction/Functions/BFL_Functions.F_Game bullet hit sound effects`))) Surface)))

(fn `Received_Notify`
  (params (MeshComp :type "SkeletalMeshComponent Object Reference") (Animation :type "AnimSequenceBase Object Reference") (EventReference :type "AnimNotifyEventReference Structure (by ref)"))
  (returns (ReturnValue :type Boolean))
  (bind _asbp_enemy (cast `/Game/SurvivlaHorrorAction/Enemys/BP_Enemy` (`ActorComponent.GetOwner` MeshComp)))
  (for _index (range (`self.TraceCounts`))
    (bind _targetactor (`/Game/SurvivlaHorrorAction/Enemys/BP_Enemy.TargetActor` _asbp_enemy))
    (`/Engine/EditorBlueprintResources/StandardMacros.IsValid` _targetactor
      (:`Is Valid`
        (bind _returnvalue (`KismetMathLibrary.FindLookAtRotation` (`Actor.K2_GetActorLocation` _asbp_enemy) (`Actor.K2_GetActorLocation` _targetactor)))
        (bind _returnvalue_2 (+ (`Actor.K2_GetActorLocation` _asbp_enemy) (+ (* (`KismetMathLibrary.GetForwardVector` _returnvalue) (`self.Forward`)) (* (`KismetMathLibrary.GetRightVector` _returnvalue) (`self.Right`)) (* (`KismetMathLibrary.GetUpVector` _returnvalue) (`self.Up`)))))
        (bind _outhits (`KismetSystemLibrary.SphereTraceMulti` _returnvalue_2 (+ _returnvalue_2 (* (`KismetMathLibrary.GreaterGreater_VectorRotator` (`KismetMathLibrary.Conv_RotatorToVector` _returnvalue) (`KismetMathLibrary.MakeRotator` 0.0 0.0 (+ (* (`KismetMathLibrary.Conv_IntToDouble` _index) (`self.TraceAngle`)) (+ (/ (* (`KismetMathLibrary.Conv_IntToDouble` (- (`self.TraceCounts`) 1)) (`self.TraceAngle`)) -2.0) (`self.AdditionalAngle`))))) (`self.TraceDistance`))) (`self.TraceSize`) "TraceTypeQuery3" true (`|MakeArray` _asbp_enemy :!type "Actor Object Reference") (`self.Draw Debug Type`) true (struct :`R` 0.023153 :`G` 0.119538 :`B` 1.0 :`A` 1.0)))
        (for _array_element _outhits
          (bind _attacktracedhittedactors (`/Game/SurvivlaHorrorAction/Enemys/BP_Enemy.AttackTracedHittedActors` _asbp_enemy))
          (bind (_bblockinghit _binitialoverlap _time _distance _location _impactpoint _normal _impactnormal _physmat _hitactor) (`GameplayStatics.BreakHitResult` _array_element))
          (if (not (`.ReturnValue` (`BlueprintMapLibrary.Map_Find` _attacktracedhittedactors _hitactor)))
            (cast `/Game/SurvivlaHorrorAction/Demo/BP_SurvivalHorrorCharacter` _hitactor)
            (`BlueprintMapLibrary.Map_Add` _attacktracedhittedactors _hitactor _array_element))))))
  (bind _values (`BlueprintMapLibrary.Map_Values` (`/Game/SurvivlaHorrorAction/Enemys/BP_Enemy.AttackTracedHittedActors` _asbp_enemy)))
  (for _array_element_2 _values
    (bind (_bblockinghit_2 _binitialoverlap_2 _time_2 _distance_2 _location_2 _impactpoint_2 _normal_2 _impactnormal_2 _physmat_2 _hitactor_2) (`GameplayStatics.BreakHitResult` _array_element_2))
    (bind _asbp_survival_horror_character (cast `/Game/SurvivlaHorrorAction/Demo/BP_SurvivalHorrorCharacter` _hitactor_2))
    (message `/Game/SurvivlaHorrorAction/Functions/BPI_Connection.PlayTargetAnimation` _hitactor_2 (`|GetArrayItem` (`/Game/SurvivlaHorrorAction/Demo/BP_SurvivalHorrorCharacter.CounterTargetAnimationFromEnemy` _asbp_survival_horror_character) (`/Game/SurvivlaHorrorAction/Enemys/BP_Enemy.CounterIndex` _asbp_enemy))))
  (`BlueprintMapLibrary.Map_Clear` (`/Game/SurvivlaHorrorAction/Enemys/BP_Enemy.AttackTracedHittedActors` _asbp_enemy)))