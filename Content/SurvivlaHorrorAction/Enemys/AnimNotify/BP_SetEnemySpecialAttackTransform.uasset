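; Anim notify that lines up a BP_Enemy and its target, the player going by variable names, for a grab attack.
; It teleports the enemy back from the target along its forward vector by the distance stored in GrabAttackMontage at GrabRandomIndex.
; It yaws each actor toward the other with per-notify rotation offsets and overrides both scales, leaving the target's location unchanged.
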(fn `Received_Notify`
  (params (MeshComp :type "SkeletalMeshComponent Object Reference") (Animation :type "AnimSequenceBase Object Reference") (EventReference :type "AnimNotifyEventReference Structure (by ref)"))
  (returns (ReturnValue :type Boolean))
  (bind _asbp_enemy (cast `/Game/SurvivlaHorrorAction/Enemys/BP_Enemy` (`ActorComponent.GetOwner` MeshComp)))
  (bind _values (`BlueprintMapLibrary.Map_Values` (`/Game/SurvivlaHorrorAction/Enemys/BP_Enemy.GrabAttackMontage` _asbp_enemy)))
  (bind (_returnvalue_roll _returnvalue_pitch _returnvalue_yaw) (`KismetMathLibrary.BreakRotator` (`KismetMathLibrary.FindLookAtRotation` (`Actor.K2_GetActorLocation` _asbp_enemy) (`Actor.K2_GetActorLocation` (`/Game/SurvivlaHorrorAction/Enemys/BP_Enemy.TargetActor` _asbp_enemy)))))
  (`Actor.K2_SetActorTransform` _asbp_enemy (`KismetMathLibrary.MakeTransform` (+ (`Actor.K2_GetActorLocation` (`/Game/SurvivlaHorrorAction/Enemys/BP_Enemy.TargetActor` _asbp_enemy)) (* (`Actor.GetActorForwardVector` _asbp_enemy) (* (`|GetArrayItem` _values (`/Game/SurvivlaHorrorAction/Enemys/BP_Enemy.GrabRandomIndex` _asbp_enemy)) -1.0))) (`KismetMathLibrary.MakeRotator` 0.0 0.0 (+ _returnvalue_yaw (`self.EnemyAdditionalRotation`))) (`self.EnemyScale`)) false true)
  (bind _returnvalue (`Actor.K2_GetActorLocation` (`/Game/SurvivlaHorrorAction/Enemys/BP_Enemy.TargetActor` _asbp_enemy)))
  (bind (_returnvalue_roll_2 _returnvalue_pitch_2 _returnvalue_yaw_2) (`KismetMathLibrary.BreakRotator` (`KismetMathLibrary.FindLookAtRotation` _returnvalue (`Actor.K2_GetActorLocation` _asbp_enemy))))
  (`Actor.K2_SetActorTransform` (`/Game/SurvivlaHorrorAction/Enemys/BP_Enemy.TargetActor` _asbp_enemy) (`KismetMathLibrary.MakeTransform` _returnvalue (`KismetMathLibrary.MakeRotator` 0.0 0.0 (+ _returnvalue_yaw_2 (`self.PlayerAdditionalRotation`))) (`self.PlayerScale`)) false false))